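; Component that decides whether the right-hand aim is making a forward carving motion.
; IsCarvingForward projects a tip point along the aim and stores it between calls to derive tip velocity from delta time.
; It returns true when the dot product of normalized velocity and aim forward lies within the cosines of the degree limits.
; BeginPlay and Tick are unused, so tip history updates only when the function is called.
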(fn `IsCarvingForward`
  (params (RightAimPosition :type "Vector Structure") (RightAimForward :type "Vector Structure") (deltatime :type "Float (double-precision)") (AimLength :type "Float (double-precision)") (MaxDegree :type "Float (double-precision)") (MinDegree :type "Float (double-precision)"))
  (returns (IsCarvingForward :type Boolean))
  (set `self.deltatime` deltatime)
  (set `self.PrevPositionTip` (`self.CurPositionTip`))
  (set `self.CurPositionTip` (+ RightAimPosition (* RightAimForward AimLength)))
  (set `self.ForwardVector` RightAimForward)
  (return (`KismetMathLibrary.InRange_FloatFloat` (`KismetMathLibrary.Dot_VectorVector` (`KismetMathLibrary.Normal` (`self.ForwardVector`)) (`KismetMathLibrary.Normal` (/ (- (`self.CurPositionTip`) (`self.PrevPositionTip`)) (`self.deltatime`)))) (`KismetMathLibrary.DegCos` MaxDegree) (`KismetMathLibrary.DegCos` MinDegree))))