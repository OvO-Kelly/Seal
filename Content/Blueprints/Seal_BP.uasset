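; Seal actor for a carving interaction, where a brush carves into the seal surface only inside the red areas of a guide texture.
; BeginPlay creates a linear render target and feeds it, with the guide, into a tessellation material on SealCanvas.
; Carving samples the guide pixel at the UV Location, and on red draws the brush material into the render target and sets right-hand controller haptics.
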(event `self.ReceiveBeginPlay`
  (bind _guidetex (`self.Guidetex`))
  (`|ExecutionSequence`
    (:`then_0`
      (bind _returnvalue (`KismetRenderingLibrary.CreateRenderTarget2D` 1024 1024 "RTF_RGBA8" (struct :`R` 1.0 :`G` 1.0 :`B` 1.0 :`A` 1.0)))
      (bind _output_get (set `self.Render Target` _returnvalue))
      (set `Texture.SRGB` false _output_get)
      (set `TextureRenderTarget.TargetGamma` 1.0 _output_get))
    (:`then_1`
      (bind _returnvalue_2 (`KismetMaterialLibrary.CreateDynamicMaterialInstance` "/Game/HandWriting_Material/Seal_Tesselation_Mat.Seal_Tesselation_Mat"))
      (`MaterialInstanceDynamic.SetTextureParameterValue` _returnvalue_2 "Rendertarget_normal" (`self.Render Target`))
      (`MaterialInstanceDynamic.SetTextureParameterValue` _returnvalue_2 "Guidetex" (`self.Guidetex`))
      (`PrimitiveComponent.SetMaterial` (`self.SealCanvas`) 0 _returnvalue_2))
    (:`then_2`
      (bind _returnvalue_3 (`KismetMaterialLibrary.CreateDynamicMaterialInstance` "/Game/HandWriting_Material/Tool_Mat.Tool_Mat"))
      (set `self.CarvingBrush` _returnvalue_3))
    (:`then_3`
      (set `self.Guidetex_sizex` (`Texture2D.Blueprint_GetSizeX` _guidetex))
      (set `self.Guidetex_sizey` (`Texture2D.Blueprint_GetSizeY` _guidetex)))))

(fn `Carving`
  (params (Size :type "Float (double-precision)") (Location :type "Vector2D Structure"))
  (bind _size (`local.Size`))
  (bind _returnvalue (/ _size 2.0))
  (bind (_y _x) (`self.uv_to_textureuv` Location_Y (`self.Guidetex_sizey`) Location_X (`self.Guidetex_sizex`)))
  (bind _pixelcolor (`VictoryBPFunctionLibrary.Victory_GetPixelFromT2D` (`self.Guidetex`) _x _y))
  (bind _isred (`self.isRed` _pixelcolor))
  (if _isred
    (bind (_canvas _size_2 _context) (`KismetRenderingLibrary.BeginDrawCanvasToRenderTarget` (`self.Render Target`)))
    (`Canvas.K2_DrawMaterial` _canvas (`self.CarvingBrush`) (- (* _size_2 (`local.Location`)) (`KismetMathLibrary.MakeVector2D` _returnvalue _returnvalue)) (`KismetMathLibrary.MakeVector2D` _size _size) (0.0 0.0) (1.0 1.0) 0.0 (0.5 0.5))
    (`KismetRenderingLibrary.EndDrawCanvasToRenderTarget` _context)
    (`PlayerController.SetHapticsByValue` (`GameplayStatics.GetPlayerController` 0) 1.0 1.0 "Right")))

(fn `isRed`
  (params (color :type "LinearColor Structure"))
  (returns (isred :type Boolean))
  (bind (_r _g _b _a) (`KismetMathLibrary.BreakColor` color))
  (return (and (>= _r 0.8) (<= _g 0.5) (<= _b 0.5) (>= _a 0.5))))

(fn `UserConstructionScript`)

(fn `uv_to_textureuv`
  (params (location_y :type "Float (double-precision)") (texture_size_y :type Integer) (location_x :type "Float (double-precision)") (texture_size_x :type Integer))
  (returns (y :type Integer) (x :type Integer))
  (return (`KismetMathLibrary.Clamp` (`KismetMathLibrary.FFloor` (* location_y texture_size_y)) 0 (- texture_size_y 1)) (`KismetMathLibrary.Clamp` (`KismetMathLibrary.FFloor` (* location_x texture_size_x)) 0 (- texture_size_x 1))))