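; VR right-hand carving tool that follows the hand, collides with surfaces and simulates pressure when carving a Seal_BP.
; Update sweeps toward the hand transform, then slides leftover movement along the hit plane.
; Intended movement into the surface becomes pressure, which slows following while carving (otherwise it snaps) and feeds the tool material.
; Helpers trace for the seal and UV, check carve direction, and drive pressure-based haptics and throttled Niagara dust.
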(event `self.ReceiveBeginPlay`)

(event `self.ReceiveTick`
  (params (DeltaSeconds :type "Float (single-precision)")))

(fn `can_carve`
  (params (deltatime :type "Float (double-precision)") (aimlength :type "Float (double-precision)"))
  (returns (can_carve :type Boolean))
  (bind _carve_tool (`self.carve_tool`))
  (bind _iscarvingforward (`/Game/Blueprints/CanCarve_Component.IsCarvingForward` (`self.CanCarve_Component`) (`SceneComponent.K2_GetComponentLocation` _carve_tool) (`SceneComponent.GetForwardVector` _carve_tool) deltatime aimlength 60.0 20.0))
  (return _iscarvingforward))

(fn `Carving_Feedback`
  (params (Location :type "Vector Structure") (Normal :type "Vector Structure"))
  (bind _pressure (`self.Pressure`))
  (bind _returnvalue (+ (`self.Feedback_Cooldown`) (`GameplayStatics.GetWorldDeltaSeconds`)))
  ; Set haptics by pressure
  (`PlayerController.SetHapticsByValue` (`GameplayStatics.GetPlayerController` 0) _pressure _pressure "Right")
  (if (>= _returnvalue (`self.Feedback_CooldownThreshold`))
    (set `self.Feedback_Cooldown` 0.0)
    ; Dust Visual
    (bind _returnvalue_2 (`NiagaraFunctionLibrary.SpawnSystemAtLocation` "/Game/VisualEffects/NS_CarveDust.NS_CarveDust" Location))
    (`NiagaraComponent.SetVariableVec3` _returnvalue_2 "DustDirection" Normal)
    (`NiagaraComponent.SetVariableLinearColor` _returnvalue_2 "DustColor" (`self.DustEffect_ParticleColor`))
    (`NiagaraComponent.SetVariableInt` _returnvalue_2 "DustNumber" (* (`self.Pressure`) (`self.DustEffect_ParticleMax`)))
    (else
      (set `self.Feedback_Cooldown` _returnvalue))))

(fn `ClampSpeed`
  (params (pressure :type "Float (double-precision)") (NewTransform :type "Transform Structure"))
  (returns (TargetTransform :type "Transform Structure"))
  (bind _prevtransform_location (`KismetMathLibrary.BreakTransform` (`self.PrevTransform`)))
  (return (`KismetMathLibrary.MakeTransform` (+ (* pressure (`KismetMathLibrary.Normal` (- NewTransform_Location _prevtransform_location))) _prevtransform_location) NewTransform_Rotation NewTransform_Scale)))

(fn `LineTrace_R`
  (params (distance :type "Float (double-precision)"))
  (returns (HitActor :type "Actor Object Reference") (UV :type "Vector2D Structure") (Location :type "Vector Structure") (Normal :type "Vector Structure"))
  (bind _carve_tool (`self.carve_tool`))
  (bind _returnvalue (`SceneComponent.K2_GetComponentLocation` _carve_tool))
  (bind _outhit (`KismetSystemLibrary.LineTraceSingle` _returnvalue (+ _returnvalue (* (`SceneComponent.GetForwardVector` _carve_tool) (`KismetMathLibrary.Conv_DoubleToVector` distance))) "TraceTypeQuery1" true))
  (bind (_bblockinghit _binitialoverlap _time _distance _location _impactpoint _normal _impactnormal _physmat _hitactor) (`GameplayStatics.BreakHitResult` _outhit))
  (set `self.HitSeal` (`GameplayStatics.ObjectIsA` _hitactor "/Game/Blueprints/Seal_BP.Seal_BP_C"))
  (return _hitactor (`GameplayStatics.FindCollisionUV` _outhit) _location _normal))

(fn `update`
  (params (New_HandTransform :type "Transform Structure") (DeltaTime :type "Float (double-precision)") (InterpSpeed :type "Float (double-precision)"))
  (locals (IntentDistance :type "Float (double-precision)" :default 0.0))
  (bind _newtransform_location (`KismetMathLibrary.BreakTransform` (`self.NewTransform`)))
  (bind (_newtransform_location_2 _newtransform_rotation) (`KismetMathLibrary.BreakTransform` (`self.NewTransform`)))
  (bind _prevtransform_location (`KismetMathLibrary.BreakTransform` (`self.PrevTransform`)))
  (bind _prevtransform_location_2 (`KismetMathLibrary.BreakTransform` (`self.PrevTransform`)))
  (set `self.NewTransform` (`KismetMathLibrary.MakeTransform` (`KismetMathLibrary.VInterpTo` _prevtransform_location_2 New_HandTransform_Location DeltaTime (* InterpSpeed (`KismetMathLibrary.SelectFloat` 1.0 0.0 (and (`self.HitSeal`) (`self.Carving`))) (`KismetMathLibrary.FClamp` (- 1.0 (`self.Pressure`)) 1e-06))) New_HandTransform_Rotation))
  (`|ExecutionSequence`
    (:`then_0`
      (set `self.MovingVector` (- _newtransform_location _prevtransform_location))
      (bind _sweephitresult (`SceneComponent.K2_SetWorldLocationAndRotation` (`self.carve_tool`) _newtransform_location_2 _newtransform_rotation true false))
      (bind (_bblockinghit _binitialoverlap _time _distance _location _impactpoint _normal) (`GameplayStatics.BreakHitResult` _sweephitresult))
      (if _bblockinghit
        (`SceneComponent.K2_AddWorldOffset` (`self.carve_tool`) (* (`KismetMathLibrary.ProjectVectorOnToPlane` (`self.MovingVector`) _normal) (* (- 1.0 _time) (`self.SecondSweepScale`))) true false)))
    (:`then_1`
      (set `self.PrevTransform` (`SceneComponent.K2_GetComponentToWorld` (`self.carve_tool`)))
      (bind _output_get (set `local.IntentDistance` (* (`KismetMathLibrary.FMax` (`KismetMathLibrary.Dot_VectorVector` (- (0.0 0.0 0.0) _normal) (`self.MovingVector`))) (`KismetMathLibrary.SelectFloat` 1.0 0.0 (and (`self.Carving`) (`self.HitSeal`))))))
      (bind _output_get_2 (set `self.Pressure` (`KismetMathLibrary.FClamp` (/ _output_get (`self.MaxIntentDistance`)))))
      (`MeshComponent.SetScalarParameterValueOnMaterials` (`self.carve_tool`) "Pressure" _output_get_2))))

(fn `UserConstructionScript`)