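; OCR text-recognition Blueprint that runs an ONNX model on a texture and returns a string, decoded through a Chinese character dictionary.
; BeginPlay loads the model with CUDA and adds a texture processor; InferModel resizes the input to a float buffer, binds tensors and runs inference.
; Postprocessing takes each step's argmax, skips index 0 and stops appending once the last "unknown" class appears.
; Unwired EventGraph chains hold usage examples and debug helpers.
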(event `self.ReceiveBeginPlay`
  ; Init process, once per object initialization
  (`self.Model_Init`)
  (bind _returnvalue (`AddComponent|NODE_AddTextureProcessFloatComponent-3` :`destinationWidth` (`self.Input_Width`) :`destinationHeight` 48))
  (set `self.Texture Processor` _returnvalue))

(fn `Bind_InputTensor`
  (bind _inputtensorsinfo (`OnnxModelWrapper.getInputTensorsInfo` (`self.Onnx Model`)))
  (bind (_name _sizeinbytes _shape _datatype) (break `OnnxTensorInfo` (`|GetArrayItem` _inputtensorsinfo)))
  (`OnnxModelWrapper.bindInputFloatArray` (`self.Onnx Model`) (`OnnxUtilityLibrary.constructOnnxTensorInfo` _name (`|MakeArray` (`KismetMathLibrary.Conv_IntToInt64` (`self.Batch size`)) (`|GetArrayItem` _shape 1) (`|GetArrayItem` _shape 2) (`KismetMathLibrary.Conv_IntToInt64` (`self.Input_Width`))) _datatype) (`self.Input Buffer`)))

(fn `Bind_OutputTensor`
  (bind _rec_length (`self.rec_length`))
  (bind _batch_size (`self.Batch size`))
  (bind _output_buffer (`self.Output Buffer`))
  (bind _outputtensorsinfo (`OnnxModelWrapper.getOutputTensorsInfo` (`self.Onnx Model`)))
  (bind (_name _sizeinbytes _shape _datatype) (break `OnnxTensorInfo` (`|GetArrayItem` _outputtensorsinfo)))
  (bind _output (`|GetArrayItem` _shape 2))
  (`KismetArrayLibrary.Array_Resize` _output_buffer (* _batch_size _rec_length (`KismetMathLibrary.Conv_Int64ToInt` _output)))
  (`OnnxModelWrapper.bindOutputFloatArray` (`self.Onnx Model`) (`OnnxUtilityLibrary.constructOnnxTensorInfo` _name (`|MakeArray` (`KismetMathLibrary.Conv_IntToInt64` _batch_size) (`KismetMathLibrary.Conv_IntToInt64` _rec_length) _output) _datatype) _output_buffer))

(fn `Infer_Model`
  (params (print_index :type Boolean) (Input_Texture :type "Texture Object Reference"))
  (returns (result :type String) (unkown_detect :type Boolean))
  (set `self.Input Texture` Input_Texture)
  (`self.Bind_OutputTensor`)
  (`self.Read_TextureNPreprocess`)
  (`self.Bind_InputTensor`)
  (`OnnxModelWrapper.run` (`self.Onnx Model`))
  (bind _result (`self.Postprocess_logits` print_index))
  (bind (_ch_result _unknown_detected) (`self.Read_dict` _result))
  (set `self.detect_unknown` false)
  (return _ch_result _unknown_detected))

(fn `Model_Init`
  (bind _returnvalue (`|GenericCreateObject` self "/Script/OnnxRuntimeNNEngine.OnnxModelWrapper"))
  (bind _output_get (set `self.Onnx Model` _returnvalue))
  (`OnnxModelWrapper.init` _output_get (`KismetStringLibrary.Concat_StrStr` (`KismetSystemLibrary.GetProjectContentDirectory`) (`self.model_name`)) "GPU_CUDA" 0 "Basic"))

(fn `Postprocess_logits`
  (params (print_result :type Boolean :default true))
  (returns (result :type "Array of Integer"))
  (bind _vector_length (`self.vector_length`))
  (for _index (range (`self.rec_length`))
    (for _index_2 (range _vector_length)
      (`KismetArrayLibrary.Array_Append` (`self.temBuffer`) (`|MakeArray` (`|GetArrayItem` (`self.Output Buffer`) (+ (* _vector_length _index) _index_2)))))
    (bind _tembuffer (`self.Append_Max_Indices`)
      (:`then`
        _)
      (:`else`
        _))
    (`KismetArrayLibrary.Array_Clear` _tembuffer))
  (if print_result
    (for _array_element (`self.max_indices`)
      (`KismetSystemLibrary.PrintString` (`KismetStringLibrary.Conv_IntToString` _array_element))))
  (return (`self.max_indices`)))

(fn `Read_dict`
  (params (Array :type "Array of Integer"))
  (returns (CH_result :type String) (unknown_detected :type Boolean))
  (for _array_element Array
    (set `self.CH_Result` (`KismetStringLibrary.Concat_StrStr` (`self.CH_Result`) (`KismetStringLibrary.GetSubstring` (`self.CH_Dict_Map`) (- _array_element 1)))))
  (return (`self.CH_Result`) (`self.detect_unknown`)))

(fn `Read_TextureNPreprocess`
  (bind _outputrawimage (`TextureProcessFloatComponent.resize` (`self.Texture Processor`) (`self.Input Texture`) false "None" true))
  (set `self.Input Buffer` _outputrawimage))

(fn `UserConstructionScript`)