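; Drawable canvas actor that collects brush strokes on a wide render target and reads the text on it with OCR.
; BeginPlay binds the render target to a dynamic material on a plane, and Draw stamps a brush material at normalized positions.
; InferOCR spawns a temporary OCR_ModelRT actor to print the recognized result.
; It can also clear the canvas, export numbered PNGs, and fade the material over Tick.
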(event `self.ReceiveBeginPlay`
  (`|ExecutionSequence`
    (:`then_0`
      (bind _returnvalue (`KismetRenderingLibrary.CreateRenderTarget2D` 3360 500 "RTF_RGBA8" (struct :`R` 1.0 :`G` 1.0 :`B` 1.0 :`A` 1.0)))
      (set `self.Render Target` _returnvalue))
    (:`then_1`
      (bind _returnvalue_2 (`KismetMaterialLibrary.CreateDynamicMaterialInstance` "/Game/HandWriting_Material/Canvas_Mat.Canvas_Mat"))
      (`MaterialInstanceDynamic.SetTextureParameterValue` _returnvalue_2 "Rendertarget" (`self.Render Target`))
      (`PrimitiveComponent.SetMaterial` (`self.Canvas`) 0 _returnvalue_2)
      (set `self.Canvas_Mat` _returnvalue_2))
    (:`then_2`
      (bind _returnvalue_3 (`KismetMaterialLibrary.CreateDynamicMaterialInstance` "/Game/HandWriting_Material/Brush_Mat.Brush_Mat"))
      (set `self.Brush_Mat` _returnvalue_3))))

(event `self.ReceiveTick`
  (params (DeltaSeconds :type "Float (single-precision)"))
  (if (`self.FadingFlag`)
    (`self.canvas_fade` DeltaSeconds)))

(event `CaptureRT`
  (bind _result (`/Engine/EditorBlueprintResources/StandardMacros.IncrementInt` (`self.Save_Num`))
    (:`  `
      (`KismetRenderingLibrary.ExportRenderTarget` (`self.Render Target`) (`KismetStringLibrary.Concat_StrStr` (`KismetSystemLibrary.GetProjectContentDirectory`) (`self.Save_Folder`)) (`KismetStringLibrary.Concat_StrStr` (`KismetStringLibrary.Concat_StrStr` "Written_" (`KismetStringLibrary.Conv_IntToString` _result)) ".png")))))

(fn `canvas_fade`
  (params (deltatime :type "Float (double-precision)"))
  (bind _canvas_mat (`self.Canvas_Mat`))
  (bind _returnvalue (`MaterialInstanceDynamic.K2_GetScalarParameterValue` _canvas_mat "Fade"))
  (`MaterialInstanceDynamic.SetScalarParameterValue` _canvas_mat "Fade" (+ _returnvalue (* deltatime (`self.FadePower`)))))

(fn `clear_canvas`
  (`KismetRenderingLibrary.ClearRenderTarget2D` (`self.Render Target`) (struct :`R` 1.0 :`G` 1.0 :`B` 1.0 :`A` 1.0)))

(fn `Draw`
  (params (Size :type "Float (double-precision)") (Location :type "Vector2D Structure"))
  (bind _size (`local.Size`))
  (bind _returnvalue (/ _size 2.0))
  (bind (_canvas _size_2 _context) (`KismetRenderingLibrary.BeginDrawCanvasToRenderTarget` (`self.Render Target`)))
  (`Canvas.K2_DrawMaterial` _canvas (`self.Brush_Mat`) (- (* _size_2 (`local.Location`)) (`KismetMathLibrary.MakeVector2D` _returnvalue _returnvalue)) (`KismetMathLibrary.MakeVector2D` _size _size) (0.0 0.0) (1.0 1.0) 0.0 (0.5 0.5))
  (`KismetRenderingLibrary.EndDrawCanvasToRenderTarget` _context))

(fn `InferOCR`
  (bind _render_target (`self.Render Target`))
  (bind _returnvalue (`|SpawnActorFromClass` "/Game/Blueprints/OCR_ModelRT.OCR_ModelRT_C" (`self.OCR_Actor_Transform`) "Undefined" "MultiplyWithRoot" null "/model.onnx" null))
  (if (`KismetSystemLibrary.IsValid` _render_target)
    (bind _result (`/Game/Blueprints/OCR_ModelRT.Infer_Model` _returnvalue false _render_target))
    (if (`KismetStringLibrary.IsEmpty` _result)
      (`KismetSystemLibrary.PrintString` "Nothing Detected")
      (else
        (`KismetSystemLibrary.PrintString` _result)))
    (`self.K2_DestroyActor` _returnvalue)
    (else
      (`KismetSystemLibrary.PrintString` "Invalid Render Target"))))

(fn `Start_Fading`
  (params (power :type "Float (double-precision)"))
  (set `self.FadingFlag` true)
  (set `self.FadePower` power))

(fn `UserConstructionScript`
  (bind _returnvalue (`AddComponent|NODE_AddStaticMeshComponent-0`))
  (bind _output_get (set `self.Canvas` _returnvalue))
  (`StaticMeshComponent.SetStaticMesh` _output_get "/Engine/BasicShapes/Plane.Plane"))