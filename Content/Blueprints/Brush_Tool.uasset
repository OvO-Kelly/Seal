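; Brush tool Blueprint that follows a supplied hand transform and reports where it points on a surface's UV map, apparently for handwriting.
; Update moves the Brush component to the hand's location and rotation.
; LineTraceR traces complex collision along the brush's forward vector, returning the hit actor and its channel 0 UV.
; While the handwriting trigger is on, that UV is interpolated from the previous one to smooth strokes.
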(fn `GetSmoothBrush_UV`
  (params (RawUV :type "Vector2D Structure") (DeltaTime :type "Float (double-precision)") (InterpSpeed :type "Float (double-precision)") (HandwritingTrigger :type Boolean))
  (returns (NewUV :type "Vector2D Structure"))
  (if HandwritingTrigger
    (return (`KismetMathLibrary.Vector2DInterpTo` (`self.PrevUV`) RawUV DeltaTime InterpSpeed))
    (else
      (return RawUV))))

(fn `LineTrace_R`
  (params (Distance :type "Float (double-precision)") (DeltaTIme :type "Float (double-precision)") (InterpSpeed :type "Float (double-precision)") (HandwrittingTrigger :type Boolean))
  (returns (HitActor :type "Actor Object Reference") (UV :type "Vector2D Structure"))
  (bind _brush (`self.Brush`))
  (bind _returnvalue (`SceneComponent.K2_GetComponentLocation` _brush))
  (bind _outhit (`KismetSystemLibrary.LineTraceSingle` _returnvalue (+ _returnvalue (* (`SceneComponent.GetForwardVector` _brush) (`KismetMathLibrary.Conv_DoubleToVector` Distance))) "TraceTypeQuery1" true))
  (bind _newuv (`self.GetSmoothBrush_UV` (`GameplayStatics.FindCollisionUV` _outhit) DeltaTIme InterpSpeed HandwrittingTrigger))
  (bind _output_get (set `self.PrevUV` _newuv))
  (return (`.HitActor` (`GameplayStatics.BreakHitResult` _outhit)) _output_get))

(fn `update`
  (params (NewHand :type "Transform Structure"))
  (`SceneComponent.K2_SetWorldLocationAndRotation` (`self.Brush`) NewHand_Location NewHand_Rotation false false))

(fn `UserConstructionScript`)